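; Enemy hazard actor that kills the TopDownCharacter when it overlaps the actor.
; On BeginPlay, a Moving timeline drives the relative location of its Sphere component without sweep.
; The timeline's Update output also feeds a two-second Delay that flips IsLooped to alternate between Play and Reverse, moving the sphere back and forth.
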(event `self.ReceiveBeginPlay`
  (bind (_direction _moving) (`Timeline|Moving` :!label _label)
    (:`Update`
      (`SceneComponent.K2_SetRelativeLocation` (`self.Sphere`) _moving false false)
      (`KismetSystemLibrary.Delay` 2.0)
      (if (`self.IsLooped`)
        (set `self.IsLooped` false)
        (goto _label :!via `Reverse`)
        (else
          (set `self.IsLooped` true)
          (goto _label))))))

(event `self.ReceiveActorBeginOverlap`
  (params (OtherActor :type "Actor Object Reference"))
  (bind _astop_down_character (cast `/Game/Blueprints/TopDownCharacter` OtherActor))
  (`/Game/Blueprints/TopDownCharacter.Death` _astop_down_character))

(fn `UserConstructionScript`)