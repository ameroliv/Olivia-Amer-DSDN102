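; Enemy Blueprint that kills the TopDownCharacter on overlap by calling its Death function, after printing a debug message.
; BeginPlay only sets the play rate of the Moving timeline.
; A timeline chain meant to lerp the Sphere's relative location and alternate play and reverse after a delay is present but never runs.
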(event `self.ReceiveBeginPlay`
  (`TimelineComponent.SetPlayRate` (`self.Moving`) (`self.New Rate`)))

(event `self.ReceiveActorBeginOverlap`
  (params (OtherActor :type "Actor Object Reference"))
  (bind _astop_down_character (cast `/Game/Blueprints/TopDownCharacter` OtherActor))
  (`KismetSystemLibrary.PrintString` "Hello")
  (`/Game/Blueprints/TopDownCharacter.Death` _astop_down_character))

(fn `UserConstructionScript`)