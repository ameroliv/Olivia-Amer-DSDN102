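; Enemy actor that patrols along a path and kills the top-down player character on contact.
; The construction script builds two relative control points from Location1 and Location2 for an InterpToMovement component and applies the Duration variable, so the path and timing come from variables.
; Any overlap with a TopDownCharacter calls that character's Death function.
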(event `self.ReceiveActorBeginOverlap`
  (params (OtherActor :type "Actor Object Reference"))
  (bind _astop_down_character (cast `/Game/Blueprints/TopDownCharacter` OtherActor))
  (`/Game/Blueprints/TopDownCharacter.Death` _astop_down_character))

(fn `UserConstructionScript`
  (bind _interptomovement (`self.InterpToMovement`))
  (set `InterpToMovementComponent.ControlPoints` (`|MakeArray` (make `InterpControlPoint` (`self.Location1`)) (make `InterpControlPoint` (`self.Location2`))) _interptomovement)
  (set `InterpToMovementComponent.Duration` (`self.duration`) _interptomovement))